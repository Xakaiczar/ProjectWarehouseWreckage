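; BP_Prop is a prop actor that can report whether it has fallen, either by leaving a bounding box or by tilting too far.
; HasFallen combines a per-axis world location check against caller-supplied bounds with a tilt check on absolute roll and pitch.
; The tilt band mirrors ToppleTilt within a 180 or 360 degree range, chosen by IsSameUpsideDown, and InvertTilt flips the result.
; BeginPlay caches the mesh's default material.
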(event EventBeginPlay
  (Variables|Default|SetDefaultMaterial (Rendering|Material|GetMaterial (Variables|Debug|GetStaticMeshComponent self) 0)))

(event Collision|EventActorBeginOverlap
  (params (OtherActor :type Actor%20Object%20Reference)))

(event EventTick
  (params (DeltaSeconds :type Float%20%28single-precision%29)))

(fn ConstructionScript)

(fn HasFallen
  (params (HighBounds :type Vector) (LowBounds :type Vector))
  (return (or (CallFunction|HasFallenOutOfBounds HighBounds LowBounds) (CallFunction|HasTiltedTooFar))))

(fn GetTiltBounds
  (params (Angle :type Float%20%28double-precision%29))
  (bind _toppletilt (Variables|Default|GetToppleTilt))
  (bind _returnvalue (Math|Float|%(Float) _toppletilt Angle))
  (bind _returnvalue_2 (- 3.6e+02 _toppletilt))
  (bind _returnvalue_3 (Math|Float|%(Float) _returnvalue_2 Angle))
  (return (Math|Float|Min(Float) _returnvalue _returnvalue_3) (Math|Float|Max(Float) _returnvalue _returnvalue_3)))

(fn HasTiltedTooFar
  (bind _returnvalue (Transformation|GetActorTransform))
  (bind _returnvalue_2 (Math|Transform|TransformRotation _returnvalue "0, 0, 0"))
  (bind _returnvalue_3 (Math|Float|Absolute(Float) (.roll _returnvalue_2)))
  (bind _returnvalue_4 (Math|Float|Absolute(Float) (.pitch _returnvalue_2)))
  (bind _angle (CallFunction|GetTiltAngle))
  (return (Class|KismetMathLibrary|XORBoolean (or (and (> _returnvalue_3 (.MinTilt (CallFunction|GetTiltBounds _angle))) (< _returnvalue_3 (.MaxTilt (CallFunction|GetTiltBounds _angle)))) (and (> _returnvalue_4 (.MinTilt (CallFunction|GetTiltBounds _angle))) (< _returnvalue_4 (.MaxTilt (CallFunction|GetTiltBounds _angle))))) (Variables|Default|GetInvertTilt))))

(fn HasFallenOutOfBounds
  (params (HighBounds :type Vector) (LowBounds :type Vector))
  (bind _returnvalue (Transformation|GetActorTransform))
  (bind _returnvalue_2 (Math|Transform|TransformLocation _returnvalue "0, 0, 0"))
  (return (Math|Boolean|ORBoolean (> (.x _returnvalue_2) (.x HighBounds)) (> (.y _returnvalue_2) (.y HighBounds)) (> (.z _returnvalue_2) (.z HighBounds)) (< (.x _returnvalue_2) (.x LowBounds)) (< (.y _returnvalue_2) (.y LowBounds)) (< (.z _returnvalue_2) (.z LowBounds)))))

(fn GetTiltAngle
  (if (Variables|Default|GetIsSameUpsideDown)
    (return 1.8e+02)
    (else
      (return 3.6e+02))))
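; BP_Barrel is a barrel actor that detects whether it has tipped over.
; HasFallen treats it as fallen when the absolute roll or pitch of its world rotation lies between 45 and 315 degrees.
; Tick calls this check every frame and prints the barrel's display name with a Fallen or Upright status, with no other gameplay effect in the graphs.
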(event EventBeginPlay)

(event Collision|EventActorBeginOverlap
  (params (OtherActor :type Actor%20Object%20Reference)))

(event EventTick
  (params (DeltaSeconds :type Float%20%28single-precision%29))
  (bind _self self)
  (bind _returnvalue (Utilities|GetDisplayName _self))
  (bind _returnvalue_2 (CallFunction|HasFallen))
  (if _returnvalue_2
    (Development|PrintString (Utilities|String|Append _returnvalue ": Fallen"))
    (else
      (Development|PrintString (Utilities|String|Append _returnvalue ": Upright")))))

(fn ConstructionScript)

(fn HasFallen
  (bind _returnvalue (Transformation|GetActorTransform))
  (bind _returnvalue_2 (Math|Transform|TransformRotation _returnvalue "0, 0, 0"))
  (bind _returnvalue_3 (Math|Float|Absolute(Float) (.roll _returnvalue_2)))
  (bind _returnvalue_4 (Math|Float|Absolute(Float) (.pitch _returnvalue_2)))
  (return (or (and (> _returnvalue_3 45.0) (< _returnvalue_3 315.0)) (and (> _returnvalue_4 45.0) (< _returnvalue_4 315.0)))))